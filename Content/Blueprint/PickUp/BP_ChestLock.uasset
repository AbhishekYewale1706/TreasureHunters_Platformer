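; BP_ChestLock is a locked chest pickup that rewards the player who reaches it holding a chest key.
; When a BP_Player_01 overlaps its box and has Chestkey set, the flipbook switches to the open chest.
; A DoOnce then limits the opening sound and the coin and gem reward, added directly to the player's totals, to a single time.
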(event OnComponentBeginOverlap(Box)
  (params (OverlappedComponent :type Primitive%20Component%20Object%20Reference) (OtherActor :type Actor%20Object%20Reference) (OtherComp :type Primitive%20Component%20Object%20Reference) (OtherBodyIndex :type Integer) (bFromSweep :type Boolean) (SweepResult :type Hit%20Result%20Structure%20%28by%20ref%29))
  (bind _asbp_player_01 (Utilities|Casting|CastToBP_Player_01 OtherActor))
  (if (Variables|/Game/Blueprint/Player/BP_Player_01.BP_Player_01_C|Getchestkey _asbp_player_01)
    (Sprite|SetFlipbook (Variables|Default|GetPaperFlipbook) "/Game/InGame_Asset/FlipBook/Objects/Chest_Open.Chest_Open")
    (Utilities|FlowControl|DoOnce false
      (:Completed
        (Audio|PlaySound2D "/Game/Sound/SW_Chestopen.SW_Chestopen" 1.0 1.0 0.0 0 0)
        (Variables|/Game/Blueprint/Player/BP_Player_01.BP_Player_01_C|SetTotal_Coins _asbp_player_01 (+ (Variables|/Game/Blueprint/Player/BP_Player_01.BP_Player_01_C|GetTotal_Coins _asbp_player_01) 10))
        (Variables|/Game/Blueprint/Player/BP_Player_01.BP_Player_01_C|SetTotal_Gems _asbp_player_01 (+ (Variables|/Game/Blueprint/Player/BP_Player_01.BP_Player_01_C|GetTotal_Gems _asbp_player_01) 10))))))

(event EventBeginPlay)

(event Collision|EventActorBeginOverlap
  (params (OtherActor :type Actor%20Object%20Reference)))

(event EventTick
  (params (DeltaSeconds :type Float%20%28single-precision%29)))

(fn ConstructionScript)