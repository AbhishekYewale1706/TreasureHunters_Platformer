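; One-way platform Blueprint that is solid only while the player is above it, letting them pass through from below.
; Every Tick, Yesplayer compares the BP_Player_01 location, lowered by a fixed vertical offset, against the platform's own height.
; It enables query and physics collision on the Box component when the player is higher and disables it otherwise.
; Only player 0 is checked, and the collision change applies to every actor.
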(event EventBeginPlay)

(event Collision|EventActorBeginOverlap
  (params (OtherActor :type Actor%20Object%20Reference)))

(event EventTick
  (params (DeltaSeconds :type Float%20%28single-precision%29))
  (CallFunction|Yesplayer))

(fn ConstructionScript)

(fn Yesplayer
  (bind _asbp_player_01 (Utilities|Casting|CastToBP_Player_01 (Game|GetPlayerCharacter 0)))
  (if (> (- (.z (Transformation|GetActorLocation _asbp_player_01)) 75.0) (.z (Transformation|GetActorLocation)))
    (Collision|SetCollisionEnabled (Variables|Default|GetBox) "QueryAndPhysics")
    (else
      (Collision|SetCollisionEnabled (Variables|Default|GetBox) "NoCollision"))))