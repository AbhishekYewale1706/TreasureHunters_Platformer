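; BP_BossEnemy2 is a boss enemy Blueprint that configures values on top of its parent class's logic.
; On BeginPlay it runs the parent logic, then sets its health (the `Heath` variable) and its death flipbook animation.
; A Sphere overlap with BP_Player_01 only prints a debug string, and Tick and ActorBeginOverlap are disabled stubs.
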(event OnComponentBeginOverlap(Sphere)
  (params (OverlappedComponent :type Primitive%20Component%20Object%20Reference) (OtherActor :type Actor%20Object%20Reference) (OtherComp :type Primitive%20Component%20Object%20Reference) (OtherBodyIndex :type Integer) (bFromSweep :type Boolean) (SweepResult :type Hit%20Result%20Structure%20%28by%20ref%29))
  (Utilities|Casting|CastToBP_Player_01 OtherActor)
  (Development|PrintString "Hello"))

(event EventBeginPlay
  (|CallParentFunction)
  (Variables|Default|SetHeath 2.5e+02)
  (Variables|Default|SetDeath%20Flipbook "/Game/InGame_Asset/FlipBook/BossEnemy2/BossEnemy2_death.BossEnemy2_death"))

(event Collision|EventActorBeginOverlap
  (params (OtherActor :type Actor%20Object%20Reference))
  (|CallParentFunction OtherActor) ; This node is disabled and will not be called.\nDrag off pins to build functionality.
)

(event EventTick
  (params (DeltaSeconds :type Float%20%28single-precision%29))
  (|CallParentFunction DeltaSeconds) ; This node is disabled and will not be called.\nDrag off pins to build functionality.
)

(fn ConstructionScript
  (|CallParentFunction))