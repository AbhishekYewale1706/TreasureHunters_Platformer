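; Base Paper2D boss enemy Blueprint that handles taking damage and dying.
; AnyDamage subtracts from clamped health, then either marks death and disables capsule collision, or briefly flashes the sprite red while holding a hit flag.
; Tick watches the death flag, switches to a non-looping death flipbook and destroys the actor after a short delay.
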(event Collision|EventActorBeginOverlap
  (params (OtherActor :type Actor%20Object%20Reference)))

(event EventTick
  (params (DeltaSeconds :type Float%20%28single-precision%29))
  (bind _sprite (Variables|Default|GetSprite))
  (if (Variables|Default|GetIsDead)
    (Sprite|SetFlipbook _sprite (Variables|Default|GetDeath%20Flipbook))
    (Components|Timeline|SetLooping _sprite false)
    (Utilities|FlowControl|Delay 1.0)
    (Actor|DestroyActor)))

(event Game|Damage|EventAnyDamage
  (params (Damage :type Float%20%28single-precision%29) (DamageType :type Damage%20Type%20Object%20Reference) (InstigatedBy :type Controller%20Object%20Reference) (DamageCauser :type Actor%20Object%20Reference))
  (Variables|Default|SetHeath (Math|Float|Clamp(Float) (- (Variables|Default|GetHeath) Damage) 0.0 1e+03))
  (if (and (<= (Variables|Default|GetHeath) 0.0) (not (Variables|Default|GetIsDead)))
    (Variables|Default|SetIsDead true)
    (CallFunction|DeadFunction)
    (else
      ;[1 1 1] hit
      (Variables|Default|Setishit true)
      (Sprite|SetSpriteColor (Variables|Default|GetSprite) "(R=1.000000,G=0.000000,B=0.032176,A=1.000000)")
      (Utilities|FlowControl|Delay 0.2)
      (Sprite|SetSpriteColor (Variables|Default|GetSprite) "(R=1.000000,G=1.000000,B=1.000000,A=1.000000)")
      (Utilities|FlowControl|Delay 0.5)
      (Variables|Default|Setishit false))))

(event EventBeginPlay)

(fn ConstructionScript)

(fn DeadFunction
  (Collision|SetCollisionEnabled (Variables|Collision|GetCapsuleComponent) "NoCollision"))