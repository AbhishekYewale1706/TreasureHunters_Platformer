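; BP_Projectile is a Paper2D bullet that damages regular and boss enemies, playing an attack sound when spawned.
; Damage is applied on Box end overlap, not begin, via casts to BP_EnemyBase and BP_BossEnemyBase, then it plays a hit sound and destroys itself.
; A Box hit stops flipbook looping and sets collision to block all channels.
; A Delay on Tick limits its lifetime to a few seconds.
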(event OnComponentHit(Box)
  (params (HitComponent :type Primitive%20Component%20Object%20Reference) (OtherActor :type Actor%20Object%20Reference) (OtherComp :type Primitive%20Component%20Object%20Reference) (NormalImpulse :type Vector :default "0, 0, 0") (Hit :type Hit%20Result%20Structure%20%28by%20ref%29))
  (Components|Timeline|SetLooping (Variables|Default|GetPaperFlipbook) false)
  (Collision|SetCollisionResponsetoAllChannels (Variables|Default|GetBox) "ECR_Block")
  (Utilities|FlowControl|Delay 3.0)
  (Actor|DestroyActor))

(event OnComponentEndOverlap(Box)
  (params (OverlappedComponent :type Primitive%20Component%20Object%20Reference) (OtherActor :type Actor%20Object%20Reference) (OtherComp :type Primitive%20Component%20Object%20Reference) (OtherBodyIndex :type Integer))
  (Utilities|FlowControl|Sequence
    (:then_0
      (bind _asbp_enemy_base (Utilities|Casting|CastToBP_EnemyBase OtherActor))
      (Game|Damage|ApplyDamage _asbp_enemy_base (Variables|Default|GetBullet_Damage) 0 0)
      (Audio|PlaySound2D "/Game/Sound/SW_EnemyHit.SW_EnemyHit" 1.0 1.0 0.0 0 0)
      (Actor|DestroyActor))
    (:then_1
      (bind _asbp_boss_enemy_base (Utilities|Casting|CastToBP_BossEnemyBase OtherActor))
      (Game|Damage|ApplyDamage _asbp_boss_enemy_base (Variables|Default|GetBullet_Damage) 0 0)
      (Audio|PlaySound2D "/Game/Sound/SW_EnemyHit.SW_EnemyHit" 1.0 1.0 0.0 0 0)
      (Actor|DestroyActor))))

(event EventBeginPlay
  (Audio|PlaySound2D "/Game/Sound/FB_Attack1.FB_Attack1" 1.0 0.5 0.0 0 0))

(event Collision|EventActorBeginOverlap
  (params (OtherActor :type Actor%20Object%20Reference)))

(event EventTick
  (params (DeltaSeconds :type Float%20%28single-precision%29))
  (Utilities|FlowControl|Delay 3.0)
  (Actor|DestroyActor))

(fn ConstructionScript)