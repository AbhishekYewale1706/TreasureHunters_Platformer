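; BP_Enemy4 is a Paper2D patrolling enemy that reuses Enemy2 flipbooks and sets its own health on BeginPlay.
; It constantly walks along its forward vector, turning around when its Wall component begins an overlap or its Ground component ends one, ignoring the player in both checks.
; Capsule hits against BP_Player_01 apply damage to the player.
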(event OnComponentHit(CapsuleComponent)
  (params (HitComponent :type Primitive%20Component%20Object%20Reference) (OtherActor :type Actor%20Object%20Reference) (OtherComp :type Primitive%20Component%20Object%20Reference) (NormalImpulse :type Vector :default "0, 0, 0") (Hit :type Hit%20Result%20Structure%20%28by%20ref%29))
  (bind _asbp_player_01 (Utilities|Casting|CastToBP_Player_01 OtherActor))
  (Game|Damage|ApplyDamage _asbp_player_01 (Variables|Default|Getplayer%20damage%20amount) 0 0))

(event OnComponentBeginOverlap(Wall)
  (params (OverlappedComponent :type Primitive%20Component%20Object%20Reference) (OtherActor :type Actor%20Object%20Reference) (OtherComp :type Primitive%20Component%20Object%20Reference) (OtherBodyIndex :type Integer) (bFromSweep :type Boolean) (SweepResult :type Hit%20Result%20Structure%20%28by%20ref%29))
  (Utilities|Casting|CastToBP_Player_01 OtherActor
    (:CastFailed
      (Transformation|SetActorRotation (Math|Rotator|CombineRotators (Transformation|GetActorRotation) "0.000000,180.000000,0.000000")))))

(event OnComponentEndOverlap(ground)
  (params (OverlappedComponent :type Primitive%20Component%20Object%20Reference) (OtherActor :type Actor%20Object%20Reference) (OtherComp :type Primitive%20Component%20Object%20Reference) (OtherBodyIndex :type Integer))
  (Utilities|Casting|CastToBP_Player_01 OtherActor
    (:CastFailed
      (Transformation|SetActorRotation (Math|Rotator|CombineRotators (Transformation|GetActorRotation) "0.000000,180.000000,0.000000")))))

(event EventBeginPlay
  (|CallParentFunction)
  (Variables|Default|Sethit%20flipbook "/Game/InGame_Asset/FlipBook/Enemy2/FB_Enemy2_hit.FB_Enemy2_hit")
  (Variables|Default|SetDeath%20Flipbook "/Game/InGame_Asset/FlipBook/Enemy2/FB_Enemy2_Dead.FB_Enemy2_Dead")
  (Variables|Default|Setidle%20flipbook "/Game/InGame_Asset/FlipBook/Enemy2/FB_Enemy2_attack.FB_Enemy2_attack")
  (Variables|Default|SetHeath (Variables|Default|Getenemy4Health)))

(event Collision|EventActorBeginOverlap
  (params (OtherActor :type Actor%20Object%20Reference))
  (|CallParentFunction OtherActor) ; This node is disabled and will not be called.\nDrag off pins to build functionality.
)

(event EventTick
  (params (DeltaSeconds :type Float%20%28single-precision%29))
  (|CallParentFunction DeltaSeconds)
  (Pawn|Input|AddMovementInput (Transformation|GetActorForwardVector) 1.0 false))

(fn ConstructionScript
  (|CallParentFunction))