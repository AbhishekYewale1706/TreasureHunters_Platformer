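; BP_Enemy3 is a Paper2D cannon enemy that fires projectiles while the player is within its trigger box.
; BeginPlay assigns cannon-specific hit, death and idle flipbooks.
; Box overlap starts a looping timer that spawns BP_EnemyShootball at Arrow1 and swaps IdleFlipbook to the firing animation; leaving clears the timer and restores idle.
; Capsule hits on BP_Player_01 apply PlayerDamageAmount as contact damage.
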(event OnComponentBeginOverlap(Box)
  (params (OverlappedComponent :type Primitive%20Component%20Object%20Reference) (OtherActor :type Actor%20Object%20Reference) (OtherComp :type Primitive%20Component%20Object%20Reference) (OtherBodyIndex :type Integer) (bFromSweep :type Boolean) (SweepResult :type Hit%20Result%20Structure%20%28by%20ref%29))
  (if (== OtherActor (Game|GetPlayerCharacter 0))
    (Variables|Default|Setidle%20flipbook "/Game/InGame_Asset/FlipBook/Cannon/FB_Cannon_idle.FB_Cannon_idle")
    (bind _returnvalue (Utilities|Time|SetTimerbyEvent (delegate Custom|shooting%20ball) 1.0 true))))

(event OnComponentEndOverlap(Box)
  (params (OverlappedComponent :type Primitive%20Component%20Object%20Reference) (OtherActor :type Actor%20Object%20Reference) (OtherComp :type Primitive%20Component%20Object%20Reference) (OtherBodyIndex :type Integer))
  (if (== OtherActor (Game|GetPlayerCharacter 0))
    (CallFunction|Stopshooting)
    (Variables|Default|Setidle%20flipbook "/Game/InGame_Asset/FlipBook/Cannon/FB_Cannon_idle.FB_Cannon_idle")))

(event OnComponentHit(CapsuleComponent)
  (params (HitComponent :type Primitive%20Component%20Object%20Reference) (OtherActor :type Actor%20Object%20Reference) (OtherComp :type Primitive%20Component%20Object%20Reference) (NormalImpulse :type Vector :default "0, 0, 0") (Hit :type Hit%20Result%20Structure%20%28by%20ref%29))
  (bind _asbp_player_01 (Utilities|Casting|CastToBP_Player_01 OtherActor))
  (Game|Damage|ApplyDamage _asbp_player_01 (Variables|Default|Getplayer%20damage%20amount) 0 0))

(event Custom|stopshooting
  (Utilities|Time|ClearandInvalidateTimerbyHandle (stale OnComponentBeginOverlap(Box) _returnvalue)))

(event Custom|shooting%20ball
  (bind _arrow1 (Variables|Default|GetArrow1))
  (Game|SpawnActorfromClass "/Game/Blueprint/Bullet/BP_EnemyShootball.BP_EnemyShootball_C" (Math|Transform|MakeTransform (Transformation|GetWorldLocation _arrow1) (Transformation|GetWorldRotation _arrow1) "1.000000,1.000000,1.000000") "Undefined" "MultiplyWithRoot" 0 0)
  (Variables|Default|Setidle%20flipbook "/Game/InGame_Asset/FlipBook/Cannon/FB_Cannon_Fire.FB_Cannon_Fire"))

(event EventBeginPlay
  (|CallParentFunction)
  (Variables|Default|Sethit%20flipbook "/Game/InGame_Asset/FlipBook/Cannon/FB_Cannon_Hit.FB_Cannon_Hit")
  (Variables|Default|SetDeath%20Flipbook "/Game/InGame_Asset/FlipBook/Cannon/FB_Cannon_destroy.FB_Cannon_destroy")
  (Variables|Default|Setidle%20flipbook "/Game/InGame_Asset/FlipBook/Cannon/FB_Cannon_idle.FB_Cannon_idle"))

(event Collision|EventActorBeginOverlap
  (params (OtherActor :type Actor%20Object%20Reference))
  (|CallParentFunction OtherActor) ; This node is disabled and will not be called.\nDrag off pins to build functionality.
)

(event EventTick
  (params (DeltaSeconds :type Float%20%28single-precision%29))
  (|CallParentFunction DeltaSeconds))

(fn ConstructionScript
  (|CallParentFunction))