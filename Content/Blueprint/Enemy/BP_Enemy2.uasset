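; BP_Enemy2 is a flipbook-animated patrolling enemy that damages the player on capsule hit, built on parent enemy logic.
; BeginPlay sets its hit, death and idle flipbooks; Tick moves it forward while Isattack is true, otherwise switching to an idle flipbook.
; Wall overlap or Ground end-overlap with anything except the player rotates it around and pauses movement for a few seconds before resuming.
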(event OnComponentHit(CapsuleComponent)
  (params (HitComponent :type Primitive%20Component%20Object%20Reference) (OtherActor :type Actor%20Object%20Reference) (OtherComp :type Primitive%20Component%20Object%20Reference) (NormalImpulse :type Vector :default "0, 0, 0") (Hit :type Hit%20Result%20Structure%20%28by%20ref%29))
  (bind _asbp_player_01 (Utilities|Casting|CastToBP_Player_01 OtherActor))
  (Game|Damage|ApplyDamage _asbp_player_01 (Variables|Default|Getplayer%20damage%20amount) 0 0))

(event OnComponentBeginOverlap(Wall)
  (params (OverlappedComponent :type Primitive%20Component%20Object%20Reference) (OtherActor :type Actor%20Object%20Reference) (OtherComp :type Primitive%20Component%20Object%20Reference) (OtherBodyIndex :type Integer) (bFromSweep :type Boolean) (SweepResult :type Hit%20Result%20Structure%20%28by%20ref%29))
  (Utilities|Casting|CastToBP_Player_01 OtherActor
    (:CastFailed
      (Transformation|SetActorRotation (Math|Rotator|CombineRotators (Transformation|GetActorRotation) "0.000000,180.000000,0.000000"))
      (Variables|Default|Setisattack false)
      (Utilities|FlowControl|Delay 3.0)
      (Variables|Default|Setisattack true))))

(event OnComponentEndOverlap(ground)
  (params (OverlappedComponent :type Primitive%20Component%20Object%20Reference) (OtherActor :type Actor%20Object%20Reference) (OtherComp :type Primitive%20Component%20Object%20Reference) (OtherBodyIndex :type Integer))
  (Utilities|Casting|CastToBP_Player_01 OtherActor
    (:CastFailed
      (Transformation|SetActorRotation (Math|Rotator|CombineRotators (Transformation|GetActorRotation) "0.000000,180.000000,0.000000"))
      (Variables|Default|Setisattack false)
      (Utilities|FlowControl|Delay 3.0)
      (Variables|Default|Setisattack true))))

(event EventBeginPlay
  (|CallParentFunction)
  (Variables|Default|Sethit%20flipbook (Variables|Default|GetHit%20Flipbook_0))
  (Variables|Default|SetDeath%20Flipbook (Variables|Default|GetDeath%20Flipbook_0))
  (Variables|Default|Setidle%20flipbook (Variables|Default|GetIdle%20Flipbook_0)))

(event Collision|EventActorBeginOverlap
  (params (OtherActor :type Actor%20Object%20Reference))
  (|CallParentFunction OtherActor) ; This node is disabled and will not be called.\nDrag off pins to build functionality.
)

(event EventTick
  (params (DeltaSeconds :type Float%20%28single-precision%29))
  (|CallParentFunction DeltaSeconds)
  (if (Variables|Default|Getisattack)
    (Pawn|Input|AddMovementInput (Transformation|GetActorForwardVector) 1.0 false)
    (Variables|Default|Setidle%20flipbook (Variables|Default|GetIdle%20Flipbook_0))
    (else
      (Variables|Default|Setidle%20flipbook "/Game/InGame_Asset/FlipBook/Enemy3/Idle.Idle"))))

(fn ConstructionScript
  (|CallParentFunction))