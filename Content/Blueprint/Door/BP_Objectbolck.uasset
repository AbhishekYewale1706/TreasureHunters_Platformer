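; Destructible 2D blocking object that breaks apart and removes itself once its Buttonpress flag is true.
; Tick polls the flag, which is not set within this Blueprint, then runs a chain of Delay nodes.
; After an initial wait it plays a rock-destroy sound and switches three Paper2D flipbooks to the destroyed animation in staggered sequence.
; It then disables the Box collision and destroys the actor.
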(event EventBeginPlay)

(event Collision|EventActorBeginOverlap
  (params (OtherActor :type Actor%20Object%20Reference)))

(event EventTick
  (params (DeltaSeconds :type Float%20%28single-precision%29))
  (if (Variables|Default|Getbuttonpress)
    (Utilities|FlowControl|Delay 3.0)
    (Audio|PlaySound2D "/Game/Sound/rock-destroy-6409.rock-destroy-6409" 0.1 0.1 0.0 0 0)
    (Sprite|SetFlipbook (Variables|Default|GetPaperFlipbook2) "/Game/InGame_Asset/FlipBook/Barrel/FB_boxdestoryed.FB_boxdestoryed")
    (Utilities|FlowControl|Delay 0.5)
    (Sprite|SetFlipbook (Variables|Default|GetPaperFlipbook1) "/Game/InGame_Asset/FlipBook/Barrel/FB_boxdestoryed.FB_boxdestoryed")
    (Utilities|FlowControl|Delay 0.5)
    (Sprite|SetFlipbook (Variables|Default|GetPaperFlipbook) "/Game/InGame_Asset/FlipBook/Barrel/FB_boxdestoryed.FB_boxdestoryed")
    (Collision|SetCollisionEnabled (Variables|Default|GetBox) "NoCollision")
    (Utilities|FlowControl|Delay 0.2)
    (Actor|DestroyActor)))

(fn ConstructionScript)