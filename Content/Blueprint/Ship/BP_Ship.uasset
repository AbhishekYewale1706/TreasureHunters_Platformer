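; BP_Ship is a flipbook-based ship that starts sailing once the player boards and is destroyed on collision.
; A Box1 overlap with BP_Player_01 sets Onship, which is never cleared here.
; While it is set, Tick sweeps the ship along world X by a fixed, frame-rate-dependent step and plays the helm and front flipbooks.
; A Box hit by anything but the player swaps the body flipbook, then destroys the ship after a delay.
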(event OnComponentHit(Box)
  (params (HitComponent :type Primitive%20Component%20Object%20Reference) (OtherActor :type Actor%20Object%20Reference) (OtherComp :type Primitive%20Component%20Object%20Reference) (NormalImpulse :type Vector :default "0, 0, 0") (Hit :type Hit%20Result%20Structure%20%28by%20ref%29))
  (Utilities|Casting|CastToBP_Player_01 OtherActor
    (:CastFailed
      (Sprite|SetFlipbook (Variables|Default|GetShipBody) "/Game/Assets/Ship/Ship/Hit/1_Sprite2.1_Sprite2")
      (Utilities|FlowControl|Delay 1.0)
      (Actor|DestroyActor))))

(event OnComponentBeginOverlap(Box1)
  (params (OverlappedComponent :type Primitive%20Component%20Object%20Reference) (OtherActor :type Actor%20Object%20Reference) (OtherComp :type Primitive%20Component%20Object%20Reference) (OtherBodyIndex :type Integer) (bFromSweep :type Boolean) (SweepResult :type Hit%20Result%20Structure%20%28by%20ref%29))
  (Utilities|Casting|CastToBP_Player_01 OtherActor)
  (Variables|Default|Setonship true))

(event EventBeginPlay)

(event Collision|EventActorBeginOverlap
  (params (OtherActor :type Actor%20Object%20Reference)))

(event EventTick
  (params (DeltaSeconds :type Float%20%28single-precision%29))
  (if (Variables|Default|Getonship)
    (Class|Actor|AddActorWorldTransform (Math|Conversions|ToTransform(Vector) (* (Transformation|GetActorForwardVector) "0.500000,0.000000,0.000000")) true false)
    (Components|Timeline|SetPlayRate (Variables|Default|GetShip_helm) 1.0)
    (Components|Timeline|SetPlayRate (Variables|Default|GetShip_frontpart) 1.0)
    (else
      (Components|Timeline|SetPlayRate (Variables|Default|GetShip_helm) 0.0)
      (Components|Timeline|SetPlayRate (Variables|Default|GetShip_frontpart) 0.0))))

(fn ConstructionScript)